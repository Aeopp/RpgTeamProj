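; Dungeon entrance trigger that asks for confirmation before sending the game to another level.
; When an RPGCharacter overlaps the Box, it shows a ConfirmMessageBox_BP on the RInGameHUD, creating it once and reattaching it on later overlaps.
; Yes saves to a "Temp" slot with LevelToOpen through RInGameMode, then loads that slot to make the transition.
; No removes the widget and restores game-and-UI input mode.
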(event OnComponentBeginOverlap(Box)
  (params (OverlappedComponent :type Primitive%20Component%20Object%20Reference) (OtherActor :type Actor%20Object%20Reference) (OtherComp :type Primitive%20Component%20Object%20Reference) (OtherBodyIndex :type Integer) (bFromSweep :type Boolean) (SweepResult :type Hit%20Result%20Structure%20%28by%20ref%29))
  (bind _currenthud (Variables|Default|GetCurrentHUD))
  (bind _asrpgcharacter (Utilities|Casting|CastToRPGCharacter OtherActor))
  (Variables|Default|SetOverlappedCharacter _asrpgcharacter)
  (Utilities|IsValid (Variables|Default|GetMessageBox)
    (:Is%20Valid
      (Class|RinGameHUD|AttachWidget _currenthud (Variables|Default|GetMessageBox)))
    (:Is%20Not%20Valid
      (bind _returnvalue (Class|RHUDBase|AddWidget _currenthud "/Game/UI/CommonWidgets/ConfirmMessageBox_BP.ConfirmMessageBox_BP_C"))
      (bind _asconfirm_message_box_bp (Utilities|Casting|CastToConfirmMessageBox_BP _returnvalue))
      (Variables|Default|SetMessageBox _asconfirm_message_box_bp)
      (EventDispatchers|BindEventtoOnYesClicked (Variables|Default|GetMessageBox) (delegate Custom|YesClicked))
      (EventDispatchers|BindEventtoOnNoClicked (Variables|Default|GetMessageBox) (delegate Custom|NoClicked))
      (Variables|/Game/UI/CommonWidgets/ConfirmMessageBox_BP.ConfirmMessageBox_BP_C|SetWidgetType (Variables|Default|GetMessageBox) "NewEnumerator5"))))

(event Custom|YesClicked
  (bind _leveltoopen (Variables|Default|GetLevelToOpen))
  (bind _asrin_game_mode (Utilities|Casting|CastToRInGameMode (Game|GetGameMode)))
  (Class|RinGameMode|Save _asrin_game_mode "Temp" _leveltoopen)
  (Class|RHUDBase|RemoveWidgetfromTop (Variables|Default|GetCurrentHUD))
  (if true
    (Development|PrintString _leveltoopen)
    (Class|RGameModeBase|Load _asrin_game_mode "Temp")))

(event Custom|NoClicked
  (bind _currenthud (Variables|Default|GetCurrentHUD))
  (Class|RHUDBase|RemoveWidgetfromTop _currenthud)
  (Class|RHUDBase|SetGameandUIInputMode _currenthud))

(event EventBeginPlay
  (bind _asrin_game_hud (Utilities|Casting|CastToRInGameHUD (HUD|GetHUD (Game|GetPlayerController 0))))
  (Variables|Default|SetCurrentHUD _asrin_game_hud))

(fn ConstructionScript)