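; Weapon actor for the Worrior player character, with a configurable mesh, attack power and skill particle effects.
; NewWeapon moves it to the player's FWeapon socket, sets mesh and power, registers it with the player's AnimInstanceBase, then moves it to a "back" socket location.
; Tick polls the character's Skill flag and toggles sixteen particle systems to match, checking one system's visibility to avoid repeated toggles.
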(event EventBeginPlay)

(event Collision|EventActorBeginOverlap
  (params (OtherActor :type Actor%20Object%20Reference)))

(event EventTick
  (params (DeltaSeconds :type Float%20%28single-precision%29))
  (bind _particlesystem (Variables|Default|GetParticleSystem))
  (bind _asworrior (Utilities|Casting|CastToWorrior (Game|GetPlayerCharacter 0)))
  (if (Variables|/Game/ThirdPersonCPP/Blueprints/Worrior.Worrior_C|GetSkill _asworrior)
    (if (not (Rendering|IsVisible (Variables|Default|GetParticleSystem)))
      (Rendering|ToggleVisibility (Variables|Default|GetParticleSystem1) true))
    (elif (Rendering|IsVisible _particlesystem)
      (Rendering|ToggleVisibility _particlesystem false))))

(fn ConstructionScript)

(fn NewWeapon
  (params (StaticMesh :type Static%20Mesh%20Object%20Reference) (AttacPower :type Float%20%28single-precision%29))
  (bind _returnvalue (Game|GetPlayerCharacter 0))
  (Transformation|SetActorLocation (Transformation|GetSocketLocation (Variables|/Script/Engine.Character|GetMesh (Game|GetPlayerCharacter 0)) "FWeapon") false false)
  (Components|StaticMesh|SetStaticMesh (Variables|Character|GetMesh) StaticMesh)
  (Variables|Default|SetAttackPower AttacPower)
  (bind _asanim_instance_base (Utilities|Casting|CastToAnimInstanceBase (Components|SkeletalMesh|GetAnimInstance (Variables|/Script/Engine.Character|GetMesh _returnvalue))))
  (Class|AnimInstanceBase|SetWeapon _asanim_instance_base self)
  (Utilities|Casting|CastToWorrior _returnvalue)
  (Transformation|SetActorLocation (Transformation|GetSocketLocation (Variables|Character|GetMesh) "back") false false))